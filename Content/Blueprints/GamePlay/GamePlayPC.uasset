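; GamePlayPC is the gameplay player controller that sets up the in-game HUD.
; On BeginPlay it caches the StartCharBP character (in a variable named MyPlayerController) and the WSG_PS_BP player state, printing a message if either cast fails.
; ShowGameHUD then creates the HUD widget if none is valid and adds it to the viewport.
; A FlipFlop toggle for the player state's Couching flag is left unconnected and never runs.
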(event `self.ReceiveBeginPlay`
  (`KismetSystemLibrary.PrintString` "GamePlayPC----------------------------------------" true true (struct :`G` 0.66 :`B` 1.0 :`A` 1.0) 100.0)
  (bind _asstart_char_bp (cast `/Game/Blueprints/Character/StartCharBP` (`GameplayStatics.GetPlayerCharacter` (`AdvancedSessionsLibrary.GetNetPlayerIndex` self)))
    (:`then`
      (set `self.MyPlayerController` _asstart_char_bp))
    (:`CastFailed`
      (`KismetSystemLibrary.PrintString` "Failed to cast  to StartCharBP" true true (struct :`R` 1.0 :`G` 0.010417 :`B` 0.010417 :`A` 1.0) 100.0)))
  (bind _aswsg_ps_bp (cast `/Game/Blueprints/GamePlay/WSG_PS_BP` (`self.PlayerState`))
    (:`then`
      (set `self.MyPlayerState` _aswsg_ps_bp))
    (:`CastFailed`
      (`KismetSystemLibrary.PrintString` "Failed to cast to WSG_PS_BP" true true (struct :`R` 1.0 :`G` 0.027019 :`A` 1.0) 100.0)))
  (`self.ShowGameHUD`))

(event `ShowGameHUD`
  (`/Engine/EditorBlueprintResources/StandardMacros.IsValid` (`self.GameHUD_WB`)
    (:`Is Valid`
      _)
    (:`Is Not Valid`
      (bind _returnvalue (`|CreateWidget` "/Game/Ui/GamePlay/HUD.HUD_C" self))
      (bind _output_get (set `self.GameHUD_WB` _returnvalue))))
  (`UserWidget.AddToViewport` _output_get 0))

(event `InputAction|Crouch`
  (params (Key :type "Key Structure" :default "AnyKey")))

(fn `UserConstructionScript`)