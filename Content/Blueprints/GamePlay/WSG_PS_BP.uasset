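; WSG_PS_BP, apparently a PlayerState, manages the Scar-L weapon for its assigned character.
; FSetPawn stores the character, and the construction script caches the GameInfoInstans game instance.
; FCreateScarL spawns the rifle owned by that character, attaches it to the mesh's R_S_Socket and copies weapon and mesh references onto the character.
; FDestroyScarL destroys the equipped weapon actor.
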(event `self.ReceiveBeginPlay`)

(fn `fCreateScar-L`
  (bind _mycharacter (`self.MyCharacter`))
  (bind _returnvalue (`|SpawnActorFromClass` "/Game/Actors/Scar-L.Scar-L_C" (`self.SpawnTransform`) "Undefined" "OverrideRootScale" (`self.MyCharacter`)))
  (bind _output_get (set `self.MyEquiptWeapon` _returnvalue))
  (`self.K2_AttachToComponent` _output_get (`Character.Mesh` (`self.MyCharacter`)) "R_S_Socket" "KeepRelative" "KeepRelative" "KeepRelative" true)
  (bind _mesh (`/Game/Actors/Scar-L.getMesh` (`self.MyEquiptWeapon`)))
  (set `self.MyWeaponMesh` _mesh)
  (set `/Game/Blueprints/Character/StartCharBP.MyEquiptWeapon` (`self.MyEquiptWeapon`) _mycharacter)
  (set `/Game/Blueprints/Character/StartCharBP.MyWeaponMesh` (`self.MyWeaponMesh`) _mycharacter))

(fn `fDestroyScar-L`
  (`self.K2_DestroyActor` (`self.MyEquiptWeapon`)))

(fn `fSetPawn`
  (params (Pawn :type "/Game/Blueprints/Character/StartCharBP Object Reference"))
  (set `self.MyCharacter` Pawn))

(fn `UserConstructionScript`
  (bind _asgame_info_instans (cast `/Game/Blueprints/AllLevels/GameInfoInstans` (`GameplayStatics.GetGameInstance`))
    (:`then`
      (set `self.GameInfoinstans` _asgame_info_instans))
    (:`CastFailed`
      (`KismetSystemLibrary.PrintString` "PS failed to Find GameInfoInstans" true true (struct :`G` 0.66 :`B` 1.0 :`A` 1.0) 10.0))))