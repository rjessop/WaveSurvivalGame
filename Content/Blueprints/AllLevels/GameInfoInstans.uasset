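; Game instance Blueprint that holds game-wide handlers for quitting, destroying the online session, and reporting network and travel errors.
; Error events convert the failure type to text and pass it to DisplayErrorMessage, which only prints it to screen.
; The save game check, both error-to-string functions and the server/client branch on network errors are empty stubs, so error messages are currently blank.
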(event `SaveGameCheck`
  ;[1 1 1] Check for save game
)

(event `self.HandleNetworkError`
  (params (FailureType :type "ENetworkFailure Enum" :default "NetDriverAlreadyExists") (bIsServer :type Boolean))
  ;[1 1 1] Handle Network Errors and Display
  (if bIsServer
    _
    (else
      _))
  (`self.DisplayErrorMessage` (`self.NetErrorToString` FailureType)))

(event `QuitGame`
  (params (playerControler :type "PlayerController Object Reference"))
  ;[1 1 1] Quit Game.
  (`KismetSystemLibrary.QuitGame` playerControler "Quit"))

(event `DestroySessionCaller`
  (params (PlayerController :type "PlayerController Object Reference"))
  ;[1 1 1] Destroy Session When Called
  (`DestroySessionCallbackProxy.DestroySession` PlayerController))

(event `self.HandleTravelError`
  (params (FailureType :type "ETravelFailure Enum" :default "NoLevel"))
  ;[1 1 1] Handle Tavel Errors And Display Message
  (`self.DisplayErrorMessage` (`self.TravelErrorToString` FailureType)))

(fn `NetErrorToString`
  (params (FailureType :type "ENetworkFailure Enum"))
  (returns (OutString :type String))
  (return ""))

(fn `TravelErrorToString`
  (params (FailureType :type "ETravelFailure Enum"))
  (returns (OutString :type String))
  (return ""))