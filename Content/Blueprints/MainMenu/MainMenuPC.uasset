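; Main menu player controller that manages the menu, loading and quit screens.
; On BeginPlay it caches the GameInfoInstans game instance, then shows the main menu with the mouse cursor visible.
; Each screen event creates its widget only if no valid one is stored, then adds it to the viewport.
; The quit screen event also calls QuitGame on the game instance right after displaying.
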(event `self.ReceiveBeginPlay`
  (bind _asgame_info_instans (cast `/Game/Blueprints/AllLevels/GameInfoInstans` (`GameplayStatics.GetGameInstance`)))
  (set `self.GameInfoInstans` _asgame_info_instans)
  (`self.showMainMenu`))

(event `showMainMenu`
  ;[1 1 1] show Main Menu and show mouse curser
  (set `self.MyPlayerController` (`GameplayStatics.GetPlayerController` 0))
  (`/Engine/EditorBlueprintResources/StandardMacros.IsValid` (`self.MainMenuWB`)
    (:`Is Valid`
      _)
    (:`Is Not Valid`
      (bind _returnvalue (`|CreateWidget` "/Game/Ui/MainMenu/MainMenu.MainMenu_C" (`self.MyPlayerController`)))
      (set `self.MainMenuWB` _returnvalue)))
  (`UserWidget.AddToViewport` (`self.MainMenuWB`) 0)
  (set `PlayerController.bShowMouseCursor` true (`self.MyPlayerController`)))

(event `ShowLoddingScreen`
  ;[1 1 1] Show The Loading Screen
  (`/Engine/EditorBlueprintResources/StandardMacros.IsValid` (`self.LoadingScreenWB`)
    (:`Is Valid`
      _)
    (:`Is Not Valid`
      (bind _returnvalue (`|CreateWidget` "/Game/Ui/AllLevels/LoadingScreen.LoadingScreen_C" (`GameplayStatics.GetPlayerController` 0)))
      (set `self.LoadingScreenWB` _returnvalue)))
  (`UserWidget.AddToViewport` (`self.LoadingScreenWB`) 0))

(event `ShowQuitScreen`
  ;[1 1 1] Apon a game quit request show the quit screen
  (`/Engine/EditorBlueprintResources/StandardMacros.IsValid` (`self.QuitScreenBW`)
    (:`Is Valid`
      _)
    (:`Is Not Valid`
      (bind _returnvalue (`|CreateWidget` "/Game/Ui/MainMenu/QuitScreen.QuitScreen_C" (`GameplayStatics.GetPlayerController` 0)))
      (set `self.QuitScreenBW` _returnvalue)))
  (`UserWidget.AddToViewport` (`self.QuitScreenBW`) 0)
  (`/Game/Blueprints/AllLevels/GameInfoInstans.QuitGame` (`self.GameInfoInstans`)))

(fn `UserConstructionScript`)