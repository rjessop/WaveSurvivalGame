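; Game state Blueprint for the main menu that caches references to the game instance and the menu's player controller.
; The construction script casts and stores GameInfoInstans.
; BeginPlay prints debug text with the PlayerArray count, then casts and stores player controller 0 as MainMenuPC, printing an error if that cast fails.
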(event `self.ReceiveBeginPlay`
  (`KismetSystemLibrary.PrintString` "GAMESTATE---------------------------------------------")
  (`KismetSystemLibrary.PrintString` (`KismetStringLibrary.Conv_IntToString` (`KismetArrayLibrary.Array_Length` (`self.PlayerArray`))))
  (bind _asmain_menu_pc (cast `/Game/Blueprints/MainMenu/MainMenuPC` (`GameplayStatics.GetPlayerController` 0))
    (:`then`
      (set `self.MainMenuPC` _asmain_menu_pc))
    (:`CastFailed`
      (`KismetSystemLibrary.PrintString` "Failed to cast PC" true true (struct :`R` 1.0 :`G` 0.020612 :`B` 0.040507 :`A` 1.0) 100.0))))

(fn `UserConstructionScript`
  (bind _asgame_info_instans (cast `/Game/Blueprints/AllLevels/GameInfoInstans` (`GameplayStatics.GetGameInstance`)))
  (set `self.GameInfoInstans` _asgame_info_instans))